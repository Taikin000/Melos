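; BP_Guide_GameMode is a game mode that runs a countdown timer for a side-scroller level.
; BeginPlay and RestartGame both call StartGame, which resets Timer to 120 and starts a looping one-second Clock timer by function name.
; Clock decrements Timer and, at zero, calls the game-over event dispatcher on the 2D side-scroller player character, then clears itself.
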(event Custom|Clock
  (Variables|Default|SetTimer (- (Variables|Default|GetTimer) 1))
  (if (== (Variables|Default|GetTimer) 0)
    (bind _as2dside_scroller_character (Utilities|Casting|CastTo2DSideScrollerCharacter (Game|GetPlayerCharacter 0)))
    (Default|CallGameOverEventDispatcher _as2dside_scroller_character)
    (Utilities|Time|ClearTimerbyFunctionName 0 "Clock")))

(event Custom|RestartGame
  (Utilities|StartGame))

(event EventTick
  (params (DeltaSeconds :type Float%20%28single-precision%29)))

(event EventBeginPlay
  (Utilities|StartGame))

(fn ConstructionScript)